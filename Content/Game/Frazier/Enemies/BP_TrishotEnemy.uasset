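; Enemy that chases the player tank and fires three bouncing bullets per volley from separate spawn points.
; BeginPlay caches the player and scales the cooldown timeline's play rate by BulletCooldown; Tick requests AI movement toward the player.
; Tick also drives firing through a Gate: the timeline's first update spawns the volley and closes it via DoOnce, and its finish reopens the gate and resets the DoOnce.
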(event `self.ReceiveBeginPlay`
  (`|ExecutionSequence`
    (:`then_0`
      (bind _returnvalue (`GameplayStatics.GetActorOfClass` "/Game/Game/Frazier/Player/BP_PlayerTankCharacter.BP_PlayerTankCharacter_C"))
      (set `self.Player` _returnvalue))
    (:`then_1`
      (`TimelineComponent.SetPlayRate` (`self.T_BulletCooldown`) (/ 1.0 (`self.BulletCooldown`))))))

(event `self.ReceiveTick`
  (params (DeltaSeconds :type "Float (single-precision)"))
  (`|ExecutionSequence`
    (:`then_0`
      (`|AIMoveTo` (`self.CharacterMovement`) self (0.0 0.0 0.0) (`self.Player`)))
    (:`then_1`
      (`/Engine/EditorBlueprintResources/StandardMacros.Gate` false :!label _label
        (:`Exit`
          (`Timeline|T_BulletCooldown` :!via `PlayFromStart`
            (:`Update`
              (`/Engine/EditorBlueprintResources/StandardMacros.DoOnce` false :!label _label_2
                (:`Completed`
                  (`self.CloseGate`)
                  (`|SpawnActorFromClass` "/Game/Game/Justin/BP_Bullet.BP_Bullet_C" (`SceneComponent.K2_GetComponentToWorld` (`self.BulletSpawnLocation`)) "Undefined" "MultiplyWithRoot" null 2.0 1 null)
                  (`|SpawnActorFromClass` "/Game/Game/Justin/BP_Bullet.BP_Bullet_C" (`SceneComponent.K2_GetComponentToWorld` (`self.BulletSpawnLocation1`)) "Undefined" "MultiplyWithRoot" null 2.0 1 null)
                  (`|SpawnActorFromClass` "/Game/Game/Justin/BP_Bullet.BP_Bullet_C" (`SceneComponent.K2_GetComponentToWorld` (`self.BulletSpawnLocation2`)) "Undefined" "MultiplyWithRoot" null 2.0 1 null))))
            (:`Finished`
              (`self.OpenGate`)
              (goto _label_2 :!via `Reset`))))))))

(event `OpenGate`
  (goto _label :!via `Open`))

(event `CloseGate`
  (goto _label :!via `Close`))

(fn `UserConstructionScript`)